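; BP_Block_1 is a track block for an endless runner that chains to the next block as BP_Runner moves through it.
; Its entry trigger asks BP_RunnerGM to spawn a block at SpawnPoint, while leaving EndTrigger raises the runner's score increment and destroys the block after a delay.
; Four speed triggers share one clamped multiplier on walk speed.
; A random lane-based SpawnObstacles function exists, but its calls are disconnected.
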(event OnComponentBeginOverlap(Trigger)
  (params (OverlappedComponent :type Primitive%20Component%20Object%20Reference) (OtherActor :type Actor%20Object%20Reference) (OtherComp :type Primitive%20Component%20Object%20Reference) (OtherBodyIndex :type Integer) (bFromSweep :type Boolean) (SweepResult :type Hit%20Result%20Structure%20%28by%20ref%29))
  (if (== (Utilities|GetClass OtherActor) "/Game/Blueprints/BP_Runner.BP_Runner_C")
    (bind _asbp_runner_gm (Utilities|Casting|CastToBP_RunnerGM (Game|GetGameMode)))
    (Default|SpawnNewBlock _asbp_runner_gm (Math|Conversions|ToTransform(Vector) (Transformation|GetWorldLocation (Variables|Default|GetSpawnPoint))))))

(event OnComponentEndOverlap(SpeedTrigger1)
  (params (OverlappedComponent :type Primitive%20Component%20Object%20Reference) (OtherActor :type Actor%20Object%20Reference) (OtherComp :type Primitive%20Component%20Object%20Reference) (OtherBodyIndex :type Integer))
  (bind _player (Variables|Default|GetPlayer))
  (bind _charactermovement (Variables|/Script/Engine.Character|GetCharacterMovement _player))
  ;[1 1 1] Gradually Increase Speed
  (if (== (Utilities|GetClass OtherActor) "/Game/Blueprints/BP_Runner.BP_Runner_C")
    (Variables|/Script/Engine.CharacterMovementComponent|SetMaxWalkSpeed _charactermovement (Math|Float|Clamp(Float) (* (Variables|/Script/Engine.CharacterMovementComponent|GetMaxWalkSpeed _charactermovement) 1.25) 7e+02 3.5e+03))))

(event OnComponentEndOverlap(EndTrigger)
  (params (OverlappedComponent :type Primitive%20Component%20Object%20Reference) (OtherActor :type Actor%20Object%20Reference) (OtherComp :type Primitive%20Component%20Object%20Reference) (OtherBodyIndex :type Integer))
  (bind _player (Variables|Default|GetPlayer))
  (if (== (Utilities|GetClass OtherActor) "/Game/Blueprints/BP_Runner.BP_Runner_C")
    (Variables|/Game/Blueprints/BP_Runner.BP_Runner_C|SetScore%20Incr _player (+ 5 (Variables|/Game/Blueprints/BP_Runner.BP_Runner_C|GetScore%20Incr _player)))
    (Utilities|FlowControl|Delay 1.5)
    (Actor|DestroyActor)))

(event OnComponentEndOverlap(SpeedTrigger2)
  (params (OverlappedComponent :type Primitive%20Component%20Object%20Reference) (OtherActor :type Actor%20Object%20Reference) (OtherComp :type Primitive%20Component%20Object%20Reference) (OtherBodyIndex :type Integer))
  (bind _player (Variables|Default|GetPlayer))
  (bind _charactermovement (Variables|/Script/Engine.Character|GetCharacterMovement _player))
  ;[1 1 1] Gradually Increase Speed
  (if (== (Utilities|GetClass OtherActor) "/Game/Blueprints/BP_Runner.BP_Runner_C")
    (Variables|/Script/Engine.CharacterMovementComponent|SetMaxWalkSpeed _charactermovement (Math|Float|Clamp(Float) (* (Variables|/Script/Engine.CharacterMovementComponent|GetMaxWalkSpeed _charactermovement) 1.25) 7e+02 3.5e+03))))

(event OnComponentEndOverlap(SpeedTrigger3)
  (params (OverlappedComponent :type Primitive%20Component%20Object%20Reference) (OtherActor :type Actor%20Object%20Reference) (OtherComp :type Primitive%20Component%20Object%20Reference) (OtherBodyIndex :type Integer))
  (bind _player (Variables|Default|GetPlayer))
  (bind _charactermovement (Variables|/Script/Engine.Character|GetCharacterMovement _player))
  ;[1 1 1] Gradually Increase Speed
  (if (== (Utilities|GetClass OtherActor) "/Game/Blueprints/BP_Runner.BP_Runner_C")
    (Variables|/Script/Engine.CharacterMovementComponent|SetMaxWalkSpeed _charactermovement (Math|Float|Clamp(Float) (* (Variables|/Script/Engine.CharacterMovementComponent|GetMaxWalkSpeed _charactermovement) 1.25) 7e+02 3.5e+03))))

(event OnComponentEndOverlap(SpeedTrigger4)
  (params (OverlappedComponent :type Primitive%20Component%20Object%20Reference) (OtherActor :type Actor%20Object%20Reference) (OtherComp :type Primitive%20Component%20Object%20Reference) (OtherBodyIndex :type Integer))
  (bind _player (Variables|Default|GetPlayer))
  (bind _charactermovement (Variables|/Script/Engine.Character|GetCharacterMovement _player))
  ;[1 1 1] Gradually Increase Speed
  (if (== (Utilities|GetClass OtherActor) "/Game/Blueprints/BP_Runner.BP_Runner_C")
    (Variables|/Script/Engine.CharacterMovementComponent|SetMaxWalkSpeed _charactermovement (Math|Float|Clamp(Float) (* (Variables|/Script/Engine.CharacterMovementComponent|GetMaxWalkSpeed _charactermovement) 1.25) 7e+02 3.5e+03))))

(event EventBeginPlay
  (bind _returnvalue (Actor|GetActorOfClass "/Game/Blueprints/BP_Runner.BP_Runner_C"))
  (Variables|Default|SetPlayer _returnvalue))

(event EventTick
  (params (DeltaSeconds :type Float%20%28single-precision%29)))

(fn ConstructionScript)

(fn SpawnObstacles
  (Development|PrintString (Utilities|String|ToString(Float) (Variables|Default|GetX%20Location)))
  (switch int (Math|Random|RandomIntegerinRange 0 2)
    (:0
      _)
    (:1
      (Game|SpawnActorfromClass "/Game/Blueprints/BP_Chest.BP_Chest_C" (Math|Conversions|ToTransform(Vector) (Math|Vector|MakeVector (Variables|Default|GetX%20Location) (.OutItem (Utilities|Array|Random (Variables|Default|GetLanes))) 1.7e+02)) "AdjustIfPossibleButAlwaysSpawn" 0 0))
    (:2
      (Game|SpawnActorfromClass "/Game/Blueprints/BP_Barrel_1.BP_Barrel_1_C" (Math|Conversions|ToTransform(Vector) (Math|Vector|MakeVector (Variables|Default|GetX%20Location) (.OutItem (Utilities|Array|Random (Variables|Default|GetLanes))) 1.7e+02)) "AdjustIfPossibleButAlwaysSpawn" 0 0))
    (:3
      (Game|SpawnActorfromClass "/Game/Blueprints/BP_Barrel_2.BP_Barrel_2_C" (Math|Conversions|ToTransform(Vector) (Math|Vector|MakeVector (Variables|Default|GetX%20Location) (.OutItem (Utilities|Array|Random (Variables|Default|GetLanes))) 1.7e+02)) "AdjustIfPossibleButAlwaysSpawn" 0 0)))
  (Variables|Default|SetX%20Location (+ (Variables|Default|GetX%20Location) 5e+02)))