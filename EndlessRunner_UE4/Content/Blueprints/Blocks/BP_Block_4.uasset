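; BP_Block_4 is a track block actor for a runner game that chains in the next block and removes itself once passed.
; When BP_Runner overlaps Trigger, it asks BP_RunnerGM to spawn a new block at the SpawnPoint's world location.
; When the runner leaves EndTrigger, the block destroys itself after a short delay.
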(event OnComponentBeginOverlap(Trigger)
  (params (OverlappedComponent :type Primitive%20Component%20Object%20Reference) (OtherActor :type Actor%20Object%20Reference) (OtherComp :type Primitive%20Component%20Object%20Reference) (OtherBodyIndex :type Integer) (bFromSweep :type Boolean) (SweepResult :type Hit%20Result%20Structure%20%28by%20ref%29))
  (if (== (Utilities|GetClass OtherActor) "/Game/Blueprints/BP_Runner.BP_Runner_C")
    (bind _asbp_runner_gm (Utilities|Casting|CastToBP_RunnerGM (Game|GetGameMode)))
    (Default|SpawnNewBlock _asbp_runner_gm (Math|Conversions|ToTransform(Vector) (Transformation|GetWorldLocation (Variables|Default|GetSpawnPoint))))))

(event OnComponentEndOverlap(EndTrigger)
  (params (OverlappedComponent :type Primitive%20Component%20Object%20Reference) (OtherActor :type Actor%20Object%20Reference) (OtherComp :type Primitive%20Component%20Object%20Reference) (OtherBodyIndex :type Integer))
  (if (== (Utilities|GetClass OtherActor) "/Game/Blueprints/BP_Runner.BP_Runner_C")
    (Utilities|FlowControl|Delay 1.5)
    (Actor|DestroyActor)))

(event EventBeginPlay)

(event Collision|EventActorBeginOverlap
  (params (OtherActor :type Actor%20Object%20Reference)))

(event EventTick
  (params (DeltaSeconds :type Float%20%28single-precision%29)))

(fn ConstructionScript)