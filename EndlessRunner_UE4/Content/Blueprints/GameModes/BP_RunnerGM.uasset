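; Game mode for a lane-based endless runner that runs spawning, HUD, pausing, game over and high score saving.
; BeginPlay starts music, the HUD and looping timers that randomly place obstacles and gems in random lanes at advancing X positions.
; SpawnNewBlock adds a random track block at a given transform.
; GameOver stops the player, pauses, shows the end menu and writes the score to an EndlessSave slot.
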(event Custom|Spawn%20New%20Block
  (params (Spawn%20Location :type Transform))
  (Game|SpawnActorfromClass (.OutItem (Utilities|Array|Random (Variables|Default|GetBlocks))) Spawn%20Location "AlwaysSpawn" 0 0))

(event Custom|Game%20Over
  (Audio|PlaySound2D "/Game/SFX/SW_Death.SW_Death" 0.5 1.0 0.0 0 0)
  (Pawn|Components|CharacterMovement|DisableMovement (Variables|/Script/Engine.Character|GetCharacterMovement (Variables|Default|GetPlayer)))
  (Game|SetGamePaused true)
  (Widget|RemovefromParent (Variables|Default|GetHUD))
  (bind _returnvalue (UserInterface|CreateWidget "/Game/UI/Widgets/EndGameMenu.EndGameMenu_C"))
  (UserInterface|Viewport|AddtoViewport _returnvalue 0)
  (CallFunction|HandleHighScore))

(event Custom|Increment%20Gem%20Count
  (Math|Integer|IncrementInt (Variables|Default|GetGems)
    (:%20%20
      (Default|IncrementGemCount (Variables|Default|GetHUD)))))

(event Custom|Pause%20Game
  (Game|SetGamePaused true)
  (bind _returnvalue (UserInterface|CreateWidget "/Game/UI/Widgets/PausedMenu.PausedMenu_C"))
  (UserInterface|Viewport|AddtoViewport _returnvalue 0))

(event Custom|Handle%20High%20Score
  (bind _player (Variables|Default|GetPlayer))
  (bind _score (Variables|/Game/Blueprints/Characters/BP_Runner.BP_Runner_C|GetScore _player))
  (bind _returnvalue (SaveGame|DoesSaveGameExist "HighScoreData"))
  (if _returnvalue
    (bind _returnvalue_2 (SaveGame|LoadGamefromSlot "HighScoreData"))
    (bind _output_get (Variables|Default|SetGame%20Saver _returnvalue_2))
    (bind _asendless_save (Utilities|Casting|CastToEndlessSave _output_get))
    (if (> _score (Variables|/Game/EndlessSave.EndlessSave_C|GetHighScore _asendless_save))
      (Variables|/Game/EndlessSave.EndlessSave_C|SetHighScore (stale _asendless_save_2) _score :!label _label)
      (SaveGame|SaveGametoSlot (Variables|Default|GetGame%20Saver) "HighScoreData"))
    (else
      (bind _returnvalue_3 (SaveGame|CreateSaveGameObject "/Game/EndlessSave.EndlessSave_C"))
      (bind _output_get_2 (Variables|Default|SetGame%20Saver _returnvalue_3))
      (bind _asendless_save_2 (Utilities|Casting|CastToEndlessSave _output_get_2))
      (goto _label))))

(event EventBeginPlay
  (Audio|PlaySound2D "/Game/SFX/SW_Castaways_GM.SW_Castaways_GM" 0.85 1.0 0.0 0 0)
  (bind _returnvalue (Actor|GetActorOfClass "/Game/Blueprints/Characters/BP_Runner.BP_Runner_C"))
  (bind _output_get (Variables|Default|SetPlayer _returnvalue))
  (Pawn|Components|CharacterMovement|SetMovementMode (Variables|/Script/Engine.Character|GetCharacterMovement _output_get) "MOVE_Walking" 0)
  (bind _returnvalue_2 (UserInterface|CreateWidget "/Game/UI/Widgets/InGameHUD.InGameHUD_C"))
  (bind _output_get_2 (Variables|Default|SetHUD _returnvalue_2))
  (UserInterface|Viewport|AddtoViewport _output_get_2 0)
  (Utilities|Time|SetTimerbyFunctionName 0 "Spawn Obstacles" 0.5 true)
  (Utilities|Time|SetTimerbyFunctionName 0 "Spawn Gems" 0.075 true))

(fn ConstructionScript)

(fn SpawnObstacles
  (switch int (Math|Random|RandomIntegerinRange 0 3)
    (:0
      _)
    (:1
      (Game|SpawnActorfromClass "/Game/Blueprints/Obstacles/BP_Chest.BP_Chest_C" (Math|Conversions|ToTransform(Vector) (Math|Vector|MakeVector (Variables|Default|GetObstacle%20X%20Location) (.OutItem (Utilities|Array|Random (Variables|Default|GetLanes))) 1.7e+02)) "AdjustIfPossibleButAlwaysSpawn" 0 0))
    (:2
      (Game|SpawnActorfromClass "/Game/Blueprints/Obstacles/BP_Barrel_1.BP_Barrel_1_C" (Math|Conversions|ToTransform(Vector) (Math|Vector|MakeVector (Variables|Default|GetObstacle%20X%20Location) (.OutItem (Utilities|Array|Random (Variables|Default|GetLanes))) 1.7e+02)) "AdjustIfPossibleButAlwaysSpawn" 0 0))
    (:3
      (Game|SpawnActorfromClass "/Game/Blueprints/Obstacles/BP_Barrel_2.BP_Barrel_2_C" (Math|Conversions|ToTransform(Vector) (Math|Vector|MakeVector (Variables|Default|GetObstacle%20X%20Location) (.OutItem (Utilities|Array|Random (Variables|Default|GetLanes))) 1.7e+02)) "AdjustIfPossibleButAlwaysSpawn" 0 0)))
  (Variables|Default|SetObstacle%20X%20Location (+ (Variables|Default|GetObstacle%20X%20Location) 8e+02)))

(fn SpawnGems
  (switch int (Math|Random|RandomIntegerinRange 0 1)
    (:1
      (Game|SpawnActorfromClass "/Game/Blueprints/BP_Gem.BP_Gem_C" (Math|Conversions|ToTransform(Vector) (Math|Vector|MakeVector (Variables|Default|GetGem%20X%20Location) (.OutItem (Utilities|Array|Random (Variables|Default|GetLanes))) 2e+02)) "AdjustIfPossibleButDontSpawnIfColliding" 0 0)
      (Variables|Default|SetGem%20X%20Location (+ (Variables|Default|GetGem%20X%20Location) 2.5e+02)))))