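; BP_Chest is an obstacle in a runner game that ends the game when the player runner hits it.
; On a hit from BP_Runner, it casts the game mode to BP_RunnerGM and calls GameOver.
; When BP_Runner leaves its Box trigger, the chest destroys itself after a short delay, cleaning up obstacles that have been passed.
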(event OnComponentEndOverlap(Box)
  (params (OverlappedComponent :type Primitive%20Component%20Object%20Reference) (OtherActor :type Actor%20Object%20Reference) (OtherComp :type Primitive%20Component%20Object%20Reference) (OtherBodyIndex :type Integer))
  (if (== (Utilities|GetClass OtherActor) "/Game/Blueprints/BP_Runner.BP_Runner_C")
    (Utilities|FlowControl|Delay 0.5)
    (Actor|DestroyActor)))

(event Collision|EventHit
  (params (MyComp :type Primitive%20Component%20Object%20Reference) (Other :type Actor%20Object%20Reference) (OtherComp :type Primitive%20Component%20Object%20Reference) (bSelfMoved :type Boolean) (HitLocation :type Vector :default "0, 0, 0") (HitNormal :type Vector :default "0, 0, 0") (NormalImpulse :type Vector :default "0, 0, 0") (Hit :type Hit%20Result%20Structure%20%28by%20ref%29))
  (if (== (Utilities|GetClass Other) "/Game/Blueprints/BP_Runner.BP_Runner_C")
    (bind _asbp_runner_gm (Utilities|Casting|CastToBP_RunnerGM (Game|GetGameMode)))
    (Default|GameOver _asbp_runner_gm)))

(fn ConstructionScript)